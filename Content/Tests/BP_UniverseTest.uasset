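; Test actor that smoke-tests the UniverseSubsystem economy when play begins.
; BeginPlay generates a universe from a config, initializes the economy, activates system 0, then prints economy and time info.
; After a two-second delay it prints time info again and a completion message, showing time progression.
; Price and shortage queries are present but left unconnected.
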(event EventBeginPlay
  (bind _returnvalue (Subsystems|GetUniverseSubsystem))
  (Class|UniverseSubsystem|GenerateUniverse _returnvalue (Utilities|Struct|MakeUniverseConfig 12345 500))
  (Class|UniverseSubsystem|InitializeEconomy _returnvalue)
  (Class|UniverseSubsystem|SetActiveEconomySystem _returnvalue)
  (Class|UniverseSubsystem|PrintEconomyStats _returnvalue)
  (Class|UniverseSubsystem|PrintTimeInfo _returnvalue)
  (Utilities|FlowControl|Delay 2.0)
  (Class|UniverseSubsystem|PrintTimeInfo _returnvalue)
  (Development|PrintString "Finished Econ"))

(fn ConstructionScript)